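; BP_Button is a pressure button that sinks while any actor overlaps its Box and rises back when the Box is empty.
; Each Tick nudges the Button component's relative Z within a clamped press range using MoveComponentTo.
; That height maps to PressPercentage, and OnPressed fires every tick it meets PressedThreshold, with no one-shot guard.
; OnPressed currently only prints a debug string.
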(event `self.ReceiveTick`
  (params (DeltaSeconds :type "Float (single-precision)"))
  (bind _button (`self.Button`))
  (bind _button_2 (`self.Button`))
  (bind (_relativelocation_x _relativelocation_y _relativelocation_z) (`KismetMathLibrary.BreakVector` (`SceneComponent.RelativeLocation` _button)))
  (bind (_relativelocation_x_2 _relativelocation_y_2 _relativelocation_z_2) (`KismetMathLibrary.BreakVector` (`SceneComponent.RelativeLocation` (`self.Button`))))
  (bind (_relativelocation_x_3 _relativelocation_y_3 _relativelocation_z_3) (`KismetMathLibrary.BreakVector` (`SceneComponent.RelativeLocation` _button_2)))
  (if (> (`KismetArrayLibrary.Array_Length` (`PrimitiveComponent.GetOverlappingActors` (`self.Box`) null)) 0)
    (`KismetSystemLibrary.MoveComponentTo` _button_2 (`KismetMathLibrary.MakeVector` 0.0 0.0 (`KismetMathLibrary.FClamp` (- _relativelocation_z_3 0.5) (`self.PressRangeMin`) (`self.PressRangeMax`))) (struct) false false 0.001)
    (else
      (`KismetSystemLibrary.MoveComponentTo` _button (`KismetMathLibrary.MakeVector` 0.0 0.0 (`KismetMathLibrary.FClamp` (+ _relativelocation_z 0.5) (`self.PressRangeMin`) (`self.PressRangeMax`))) (struct) false false 0.004)))
  (bind _output_get (set `self.PressPercentage` (`KismetMathLibrary.MapRangeClamped` _relativelocation_z_2 (`self.PressRangeMin`) (`self.PressRangeMax`) 1.0 0.0)))
  (if (>= _output_get (`self.PressedThreshold`))
    (`self.OnPressed`)))

(event `OnPressed`
  (`KismetSystemLibrary.PrintString` "Pressed" true true (struct :`G` 0.66 :`B` 1.0 :`A` 1.0) 10.0))

(fn `UserConstructionScript`)