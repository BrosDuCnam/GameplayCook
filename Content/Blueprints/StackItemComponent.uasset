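; StackItemComponent lets physics items stack on one another by linking their components into a vertical chain.
; TryStack traces down from its parent along local up, finds a StackItemComponent among the hit body's children, and snaps its parent to that item's StackPoint socket.
; It records up and down references, which DetachStack follows upward recursively, calling detach on each upper stack component and clearing the up link only.
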(fn `DetachStack`
  (bind _stackeditemup (`self.StackedItemUp`)
    (:`then`
      (`self.K2_DetachFromComponent` _stackeditemup "KeepWorld" "KeepWorld" "KeepWorld" true)
      (`self.DetachStack` _stackeditemup)
      (set `self.StackedItemUp` null))
    (:`else`)))

(fn `TryStack`
  (bind _returnvalue (`self.GetAttachParent`))
  (bind _returnvalue_2 (`self.K2_GetComponentLocation` _returnvalue))
  (bind (_outhit _returnvalue_3) (`KismetSystemLibrary.LineTraceSingleByProfile` :`Start` _returnvalue_2 :`End` (+ (* (`KismetMathLibrary.GetUpVector` (`self.K2_GetComponentRotation` _returnvalue)) (* (`self.StackRange`) -1.0)) _returnvalue_2) :`ProfileName` "PhysicsActor" :`DrawDebugType` "ForOneFrame"))
  (if _returnvalue_3
    (bind (_bblockinghit _binitialoverlap _time _distance _location _impactpoint _normal _impactnormal _physmat _hitactor _hitcomponent) (`GameplayStatics.BreakHitResult` _outhit))
    (if (`|EnumEquality` (`PrimitiveComponent.GetCollisionObjectType` _hitcomponent) "ECC_PhysicsBody")
      (`self.StackedItemDown`
        (:`then`)
        (:`else`
          (for _array_element (`self.GetChildrenComponents` _hitcomponent false)
            (bind _asstack_item_component (cast `/Game/Blueprints/StackItemComponent` _array_element))
            (`self.K2_AttachToComponent` (`self.GetAttachParent`) (`self.GetAttachParent` _asstack_item_component) "StackPoint" "SnapToTarget" "SnapToTarget" "KeepWorld" true)
            (set `self.StackedItemDown` _asstack_item_component)
            (set `/Game/Blueprints/StackItemComponent.StackedItemUp` self _asstack_item_component)
            (break)))))))