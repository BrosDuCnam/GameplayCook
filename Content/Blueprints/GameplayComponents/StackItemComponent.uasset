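; StackItemComponent lets physics items, including cut ones, stack on each other and detach as a group.
; TryStack traces down for another stack item, attaches to it or, if cut, to the item below it, closes the gap and snaps uncut items flat.
; Items keep up and down links.
; TryDetach recurses to the top items, then DetachStack unwinds downward, counting calls so each item waits for all those above.
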(fn `DetachStack`
  (bind _stackeditemdown (`self.StackedItemDown`))
  (if (>= (`self.NbDetachCalls`) (`KismetArrayLibrary.Array_Length` (`self.StackedItemUp`)))
    (if (not (== (`self.StackedItemDown`) null))
      (`self.K2_DetachFromComponent` (`self.GetAttachParent`) "KeepWorld" "KeepWorld" "KeepRelative" true)
      (`/Engine/EditorBlueprintResources/StandardMacros.IncrementInt` (`/Game/Blueprints/GameplayComponents/StackItemComponent.NbDetachCalls` _stackeditemdown)
        (:`  `
          (`self.DetachStack` _stackeditemdown))))
    (set `self.isStacked` false)
    (set `self.StackedItemDown` null)
    (`KismetArrayLibrary.Array_Clear` (`self.StackedItemUp`))))

(fn `TryDetach`
  (bind _stackeditemup (`self.StackedItemUp`))
  (if (<= (`KismetArrayLibrary.Array_Length` _stackeditemup) 0)
    (`self.DetachStack`)
    (else
      (for _array_element _stackeditemup
        (`self.TryDetach` _array_element)))))

(fn `TryStack`
  (locals (snapRotX :type "Float (double-precision)") (hasStacked :type Boolean) (currentStack :type "/Game/Blueprints/GameplayComponents/StackItemComponent Object Reference"))
  (bind _returnvalue (`self.GetAttachParent`))
  (bind _returnvalue_2 (`self.K2_GetComponentLocation` (`self.GetAttachParent`)))
  (if (not (`self.isStacked`))
    (set `local.hasStacked` false)
    (bind (_outhit _returnvalue_3) (`KismetSystemLibrary.LineTraceSingleByProfile` :`Start` _returnvalue_2 :`End` (+ _returnvalue_2 (* (0.0 0.0 -1.0) (`self.StackRange`))) :`ProfileName` "PhysicsActor" :`DrawTime` 20.0))
    (if _returnvalue_3
      (bind (_bblockinghit _binitialoverlap _time _distance _location _impactpoint _normal _impactnormal _physmat _hitactor _hitcomponent _hitbonename _bonename _hititem _elementindex _faceindex _tracestart) (`GameplayStatics.BreakHitResult` _outhit))
      (if (`|EnumEquality` (`PrimitiveComponent.GetCollisionObjectType` _hitcomponent) "ECC_PhysicsBody")
        (for _array_element (`self.GetChildrenComponents` _hitcomponent false)
          (bind _asstack_item_component (cast `/Game/Blueprints/GameplayComponents/StackItemComponent` _array_element))
          (if (`/Game/Blueprints/GameplayComponents/StackItemComponent.isCut` _asstack_item_component)
            (bind _stackeditemdown (`/Game/Blueprints/GameplayComponents/StackItemComponent.StackedItemDown` _asstack_item_component)
              (:`then`
                (bind _output_get (set `local.currentStack` _stackeditemdown))
                (`/Game/Blueprints/GameplayComponents/StackItemComponent.StackedItemDown` _output_get
                  (:`then`
                    _)
                  (:`else`)))
              (:`else`))
            (else
              (set `local.currentStack` _asstack_item_component)))
          (bind (_outhit_2 _returnvalue_4) (`KismetSystemLibrary.LineTraceSingleByProfile` _impactpoint _tracestart "PhysicsActor" false (`|MakeArray` (`self.GetOwner` _asstack_item_component)) "None" false (struct :`R` 1.0 :`A` 1.0) (struct :`G` 1.0 :`A` 1.0) 20.0))
          (if _returnvalue_4
            (bind _returnvalue_5 (`self.K2_AttachToComponent` _returnvalue (`self.GetAttachParent` (`local.currentStack`)) "None" "KeepWorld" "KeepWorld" "KeepWorld" true))
            (if _returnvalue_5
              (bind (_bblockinghit_2 _binitialoverlap_2 _time_2 _distance_2 _location_2 _impactpoint_2 _normal_2 _impactnormal_2 _physmat_2 _hitactor_2 _hitcomponent_2 _hitbonename_2 _bonename_2 _hititem_2 _elementindex_2 _faceindex_2 _tracestart_2) (`GameplayStatics.BreakHitResult` _outhit_2))
              (`self.K2_SetWorldLocation` _returnvalue (- (`self.K2_GetComponentLocation` _returnvalue) (- _impactpoint_2 _tracestart_2)) false true)
              (if (`self.isCut`)
                (set `local.hasStacked` true :!label _label)
                (set `self.NbDetachCalls` 0)
                (bind _output_get_2 (set `self.StackedItemDown` _asstack_item_component))
                (`KismetArrayLibrary.Array_Add` (`/Game/Blueprints/GameplayComponents/StackItemComponent.StackedItemUp` _output_get_2) self)
                (break)
                (else
                  (`|ExecutionSequence`
                    (:`then_0`
                      (if (>= (`KismetMathLibrary.DegCos` (.roll (`SceneComponent.RelativeRotation` _returnvalue))) 0.0)
                        (set `local.snapRotX` 0.0)
                        (else
                          (set `local.snapRotX` 180.0))))
                    (:`then_1`
                      (`self.K2_SetRelativeRotation` _returnvalue (`KismetMathLibrary.MakeRotator` (`local.snapRotX`) 0.0 (.yaw (`SceneComponent.RelativeRotation` _returnvalue))) false false)
                      (goto _label))))))))
        (if (`local.hasStacked`)
          (set `self.isStacked` true)
          (bind _stackeditemdown_2 (`self.StackedItemDown`)
            (:`then`
              (set `/Game/Blueprints/GameplayComponents/StackItemComponent.isStacked` true _stackeditemdown_2))
            (:`else`
              (`KismetSystemLibrary.PrintString` "Error isStacked none" true true (struct :`R` 1.0 :`G` 0.014042 :`A` 1.0) 10.0)))
          ;[1 0 0] debug
          (`KismetSystemLibrary.PrintString` "End 3")
          (`KismetSystemLibrary.PrintString` (`KismetStringLibrary.Conv_IntToString` (`KismetArrayLibrary.Array_Length` (`self.StackedItemUp`))) :!label _label_2))
        (else
          (`KismetSystemLibrary.PrintString` "End 2")
          (goto _label_2)))
      (else
        (`KismetSystemLibrary.PrintString` "END 1")
        (goto _label_2)))))