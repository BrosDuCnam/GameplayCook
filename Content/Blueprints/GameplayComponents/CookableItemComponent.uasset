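; Scene component that makes an item cook while it sits above a heat source, up to a fully cooked level.
; Each tick it traces along the parent's negative up vector within CookRange for a physics body with a child CookingItemComponent.
; That component's CookingHeat, divided by distance, accumulates into CookAmount, which maps against CookingTime to CookLevel.
; CookLevel drives the parent mesh's "Cooked" material parameter, with debug trace and print output left on.
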(event `self.ReceiveTick`
  (params (DeltaSeconds :type "Float (single-precision)"))
  (bind _returnvalue (`self.GetAttachParent`))
  (bind _cooklevel (`self.CookLevel`))
  (bind _returnvalue_2 (`self.K2_GetComponentLocation` _returnvalue))
  (bind (_outhit _returnvalue_3) (`KismetSystemLibrary.LineTraceSingleByProfile` :`Start` _returnvalue_2 :`End` (+ (* (`KismetMathLibrary.GetUpVector` (`self.K2_GetComponentRotation` _returnvalue)) (* (`self.CookRange`) -1.0)) _returnvalue_2) :`ProfileName` "PhysicsActor" :`DrawDebugType` "ForOneFrame" :`TraceColor` (struct :`G` 0.824485 :`B` 1.0 :`A` 1.0) :`TraceHitColor` (struct :`G` 0.010426 :`B` 1.0 :`A` 1.0)))
  (if _returnvalue_3
    (bind (_bblockinghit _binitialoverlap _time _distance _location _impactpoint _normal _impactnormal _physmat _hitactor _hitcomponent) (`GameplayStatics.BreakHitResult` _outhit))
    (if (`|EnumEquality` (`PrimitiveComponent.GetCollisionObjectType` _hitcomponent) "ECC_PhysicsBody")
      (for _array_element (`self.GetChildrenComponents` _hitcomponent false)
        (bind _ascooking_item_component (cast `/Game/Blueprints/GameplayComponents/CookingItemComponent` _array_element))
        (if (not (>= (`self.CookLevel`) 1.0))
          (bind _output_get (set `self.CookAmount` (+ (`self.CookAmount`) (* DeltaSeconds (/ (`/Game/Blueprints/GameplayComponents/CookingItemComponent.CookingHeat` _ascooking_item_component) (`KismetMathLibrary.FClamp` (`KismetMathLibrary.Vector_Distance` _impactpoint (`self.K2_GetComponentLocation` (`self.GetAttachParent`))) 1.0 (`self.CookRange`)))))))
          (set `self.CookLevel` (`KismetMathLibrary.MapRangeClamped` _output_get 0.0 (`self.CookingTime`) 0.0 1.0))
          (bind _asstatic_mesh_component (cast `StaticMeshComponent` (`self.GetAttachParent`)))
          (bind _returnvalue_4 (`PrimitiveComponent.CreateDynamicMaterialInstance` _asstatic_mesh_component 0 null "None"))
          (`MaterialInstanceDynamic.SetScalarParameterValue` _returnvalue_4 "Cooked" _cooklevel)
          (`KismetSystemLibrary.PrintString` (`KismetStringLibrary.Conv_DoubleToString` _cooklevel) true true (struct :`G` 0.66 :`B` 1.0 :`A` 1.0) 10.0)
          (break))))))