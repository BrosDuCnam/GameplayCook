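; Order completed area component that reads which ingredients make up a food item handed in as a completed order.
; OnOrderCompleted walks up the food's StackedItemUp chain, finding an IngredientItemComponent among each attach parent's children to collect ingredient names.
; It joins the names into a comma-separated string and only prints it.
; SetOrderDetails is an empty stub, so no comparison against an order takes place.
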(fn `OnOrderCompleted`
  (params (Food :type "/Game/Blueprints/GameplayComponents/StackItemComponent Object Reference"))
  (locals (CurrentStackItem :type "/Game/Blueprints/GameplayComponents/StackItemComponent Object Reference") (Ingredients :type "Array of String") (IngredientMessage :type String))
  (set `local.Ingredients` (`|MakeArray` ""))
  (bind _output_get (set `local.CurrentStackItem` Food))
  (bind _stackeditemup (`/Game/Blueprints/GameplayComponents/StackItemComponent.StackedItemUp` _output_get))
  (while (== _stackeditemup null)
    (for _array_element (`self.GetChildrenComponents` (`self.GetAttachParent` _stackeditemup) false)
      (bind _asingredient_item_component (cast `/Game/Blueprints/GameplayComponents/IngredientItemComponent` _array_element))
      (`KismetArrayLibrary.Array_Add` (`local.Ingredients`) (`/Game/Blueprints/GameplayComponents/IngredientItemComponent.IngredientName` _asingredient_item_component))
      (set `local.CurrentStackItem` (`/Game/Blueprints/GameplayComponents/StackItemComponent.StackedItemUp` (`local.CurrentStackItem`)))
      (break)))
  (for _array_element_2 (`local.Ingredients`)
    (set `local.IngredientMessage` (`KismetStringLibrary.Concat_StrStr` (`local.IngredientMessage`) " , " _array_element_2)))
  (`KismetSystemLibrary.PrintString` (`local.IngredientMessage`) true true (struct :`G` 0.66 :`B` 1.0 :`A` 1.0) 20.0))

(fn `SetOrderDetails`
  (params (id :type String) (ingredients :type "Array of String")))