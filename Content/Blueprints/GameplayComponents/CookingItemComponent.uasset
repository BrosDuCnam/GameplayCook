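; Component that drives a shared cooking sound based on how many items are currently cooking.
; Adding an item increments a counter and, on the first one, starts the audio at a random offset so loops do not sound identical.
; Removing an item decrements the counter and stops the audio once none remain.
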(event `AddCookingItem`
  (bind _amountcooking (`self.AmountCooking`))
  (if (== _amountcooking 0)
    (`self.PlaySound`))
  (`/Engine/EditorBlueprintResources/StandardMacros.IncrementInt` _amountcooking))

(event `PlaySound`
  (`AudioComponent.Play` (`self.Audio`) (`KismetMathLibrary.RandomFloatInRange` 0.0 93.0)))

(event `StopSound`
  (`AudioComponent.Stop` (`self.Audio`)))

(event `RemoveCookingItem`
  (bind _amountcooking (`self.AmountCooking`))
  (`/Engine/EditorBlueprintResources/StandardMacros.DecrementInt` _amountcooking
    (:`  `
      (if (<= _amountcooking 0)
        (`self.StopSound`)))))