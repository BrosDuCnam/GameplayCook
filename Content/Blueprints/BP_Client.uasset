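; BP_Client is the game's Socket.IO client actor, connecting to a server and starting the games UI once connected.
; On BeginPlay it registers itself on BP_GameInstance, binds the connected event and connects using an HTTP URL built from Ip and Port, with Type as a query parameter.
; On connection it finds BP_UISpawn's UI_base widget and calls InitGames with empty defaults rather than the session details.
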(event `self.ReceiveBeginPlay`
  (set `/Game/Blueprints/BP_GameInstance.Client` self (cast `/Game/Blueprints/BP_GameInstance` (`GameplayStatics.GetGameInstance`) :!pure true))
  (add `SocketIOClientComponent.OnConnected` (`self.SIOClient`) (delegate `On Connected`))
  (`self.Connect`))

(event `On Connected`
  (params (SocketId :type String) (SessionId :type String) (bIsReconnection :type Boolean))
  (bind _returnvalue (`GameplayStatics.GetActorOfClass` "/Game/Blueprints/UI/BP_UISpawn.BP_UISpawn_C"))
  (bind _asui_base (cast `/Game/Blueprints/UI/UI_base` (`WidgetComponent.GetWidget` (`/Game/Blueprints/UI/BP_UISpawn.Widget` _returnvalue))))
  (`/Game/Blueprints/UI/UI_base.Init_Games` _asui_base "" "" false))

(fn `Build URL`
  (returns (Url :type String))
  (return (`KismetStringLibrary.Concat_StrStr` "http://" (`self.Ip`) ":" (`self.Port`))))

(fn `Connect`
  (locals (NewLocalVar_0 :type "Map of String to String"))
  (bind _output_get (set `SocketIOClientComponent.URLParams` (make `SIOConnectParams` (`self.Build URL`) _ (`|MakeMap` "type" (`self.Type`))) (`self.SIOClient`)))
  (`SocketIOClientComponent.ConnectWithParams` (`self.SIOClient`) _output_get)
  (`KismetSystemLibrary.PrintString` "Hello"))

(fn `UserConstructionScript`)