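; BP_Command is a grabbable order ticket that displays a command ID and its list of ingredients.
; On BeginPlay it configures its GrabComponent with a fixed grab type and zero mass.
; SetCommand writes the ID with a "#" prefix to TextId, then concatenates the ingredients with dash prefixes under an "Ingredients:" label into TextIngredient.
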(event `self.ReceiveBeginPlay`
  (bind _grabcomponent (`self.GrabComponent`))
  (set `/Game/VRTemplate/Blueprints/GrabComponent.GrabType` "NewEnumerator4" _grabcomponent)
  (set `/Game/VRTemplate/Blueprints/GrabComponent.MassKg` 0.0 _grabcomponent))

(fn `set_command`
  (params (id :type String) (ingredients :type "Array of String"))
  (locals (text :type String))
  (set `local.text` "Ingredients: \n")
  (`TextRenderComponent.K2_SetText` (`self.text_id`) (`KismetTextLibrary.Conv_StringToText` (`KismetStringLibrary.Concat_StrStr` "# " id)))
  (for _array_element ingredients
    (set `local.text` (`KismetStringLibrary.Concat_StrStr` (`local.text`) "-  " _array_element " \n")))
  (`TextRenderComponent.K2_SetText` (`self.text_ingredient`) (`KismetTextLibrary.Conv_StringToText` (`local.text`)))
  (return))

(fn `UserConstructionScript`)