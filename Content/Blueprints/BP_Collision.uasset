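; BP_Collision is a cube collision actor that reports objects hitting it to a Socket.IO server as thrown-object events.
; On each hit it rescales the impact point by the cube's scale into normalized coordinates relative to the root, ignoring rotation, and prints them.
; SendCollisionInfo packs the hit actor's name, that location and the other actor's velocity into JSON, then emits "on_object_thrown" through the BP_GameInstance client.
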(event `self.ReceiveBeginPlay`)

(event `self.Cube.OnComponentHit`
  (params (HitComponent :type "PrimitiveComponent Object Reference") (OtherActor :type "Actor Object Reference") (OtherComp :type "PrimitiveComponent Object Reference") (NormalImpulse :type "Vector Structure") (Hit :type "HitResult Structure (by ref)"))
  (bind (_bblockinghit _binitialoverlap _time _distance _location _impactpoint _normal _impactnormal _physmat _hitactor) (`GameplayStatics.BreakHitResult` Hit))
  (bind _returnvalue (/ (+ (/ (/ (- _location (`SceneComponent.K2_GetComponentLocation` (`self.DefaultSceneRoot`))) (`SceneComponent.K2_GetComponentScale` (`self.Cube`))) (100.0 100.0 100.0)) (1.0 1.0 1.0)) (2.0 2.0 2.0)))
  (set `self.CollisionObject` _hitactor)
  (`KismetSystemLibrary.PrintString` (`KismetStringLibrary.Conv_VectorToString` _returnvalue) true true (struct :`G` 0.66 :`B` 1.0 :`A` 1.0) 500.0)
  (set `self.CollisionLocation` _returnvalue)
  (set `self.CollisionVelocity` (`self.GetVelocity` OtherActor))
  (`self.SendCollisionInfo`))

(fn `SendCollisionInfo`
  (bind (_x _y _z) (`KismetMathLibrary.BreakVector3f` (`self.CollisionVelocity`)))
  (bind (_x_2 _y_2 _z_2) (`KismetMathLibrary.BreakVector3f` (`self.CollisionLocation`)))
  (bind _returnvalue (`SIOJsonObject.ConstructJsonObject`))
  (`SIOJsonObject.SetStringField` _returnvalue "object_name" (`KismetStringLibrary.Conv_ObjectToString` (`self.CollisionObject`)))
  (`SIOJsonObject.SetArrayField` _returnvalue "location" (`|MakeArray` (`SIOJsonValue.ConstructJsonValueNumber` _x_2) (`SIOJsonValue.ConstructJsonValueNumber` _y_2) (`SIOJsonValue.ConstructJsonValueNumber` _z_2)))
  (`SIOJsonObject.SetArrayField` _returnvalue "velocity" (`|MakeArray` (`SIOJsonValue.ConstructJsonValueNumber` _x) (`SIOJsonValue.ConstructJsonValueNumber` _y) (`SIOJsonValue.ConstructJsonValueNumber` _z)))
  (`SocketIOClientComponent.Emit` (`/Game/Blueprints/BP_Client.SIOClient` (`/Game/Blueprints/BP_GameInstance.Client` (cast `/Game/Blueprints/BP_GameInstance` (`GameplayStatics.GetGameInstance`) :!pure true))) "on_object_thrown" (`SIOJsonValue.ConstructJsonValueObject` _returnvalue) "/"))

(fn `UserConstructionScript`)