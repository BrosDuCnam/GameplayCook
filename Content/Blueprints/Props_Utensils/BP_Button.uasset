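; BP_Button is a physical push button that sounds audio and toggles a horn over Socket.IO.
; Each tick, actors overlapping the Box sink the Button component within a clamped Z range; otherwise it rises back.
; Travel maps to a press percentage, with hysteresis: Pressed fires at a threshold, Released only at full return.
; These events start or stop the audio and emit "toggle_horn" with a boolean state through the GameInstance's client.
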(event `self.ReceiveTick`
  (params (DeltaSeconds :type "Float (single-precision)"))
  (bind _button (`self.Button`))
  (bind _button_2 (`self.Button`))
  (bind (_relativelocation_x _relativelocation_y _relativelocation_z) (`KismetMathLibrary.BreakVector` (`SceneComponent.RelativeLocation` _button)))
  (bind (_relativelocation_x_2 _relativelocation_y_2 _relativelocation_z_2) (`KismetMathLibrary.BreakVector` (`SceneComponent.RelativeLocation` (`self.Button`))))
  (bind (_relativelocation_x_3 _relativelocation_y_3 _relativelocation_z_3) (`KismetMathLibrary.BreakVector` (`SceneComponent.RelativeLocation` _button_2)))
  (if (> (`KismetArrayLibrary.Array_Length` (`PrimitiveComponent.GetOverlappingActors` (`self.Box`) null)) 0)
    (`KismetSystemLibrary.MoveComponentTo` _button_2 (`KismetMathLibrary.MakeVector` 0.0 0.0 (`KismetMathLibrary.FClamp` (- _relativelocation_z_3 0.5) (`self.PressRangeMin`) (`self.PressRangeMax`))) (struct) false false 0.001)
    (else
      (`KismetSystemLibrary.MoveComponentTo` _button (`KismetMathLibrary.MakeVector` 0.0 0.0 (`KismetMathLibrary.FClamp` (+ _relativelocation_z 0.5) (`self.PressRangeMin`) (`self.PressRangeMax`))) (struct) false false 0.004)))
  (bind _output_get (set `self.PressPercentage` (`KismetMathLibrary.MapRangeClamped` _relativelocation_z_2 (`self.PressRangeMin`) (`self.PressRangeMax`) 1.0)))
  (if (>= _output_get (`self.PressedThreshold`))
    (if (not (`self.startPress`))
      (`self.Pressed`)
      (set `self.startPress` true))
    (elif (<= (`self.PressPercentage`) 0.0)
      (if (`self.startPress`)
        (`self.Released`)
        (set `self.startPress` false)))))

(event `Pressed`
  (`AudioComponent.Play` (`self.Audio`) 0.0)
  (bind _returnvalue (`SIOJsonObject.ConstructJsonObject`))
  (`SIOJsonObject.SetBoolField` _returnvalue "state" true)
  (`SocketIOClientComponent.EmitWithGraphCallBack` (`/Game/Blueprints/ServerStuff/BP_Client.SIOClient` (`/Game/Blueprints/ServerStuff/BP_GameInstance.Client` (cast `/Game/Blueprints/ServerStuff/BP_GameInstance` (`GameplayStatics.GetGameInstance`) :!pure true))) "toggle_horn" (`SIOJsonValue.ConstructJsonValueObject` _returnvalue) "/"))

(event `Released`
  (`AudioComponent.Stop` (`self.Audio`))
  (bind _returnvalue (`SIOJsonObject.ConstructJsonObject`))
  (`SIOJsonObject.SetBoolField` _returnvalue "state" false)
  (`SocketIOClientComponent.EmitWithGraphCallBack` (`/Game/Blueprints/ServerStuff/BP_Client.SIOClient` (`/Game/Blueprints/ServerStuff/BP_GameInstance.Client` (cast `/Game/Blueprints/ServerStuff/BP_GameInstance` (`GameplayStatics.GetGameInstance`) :!pure true))) "toggle_horn" (`SIOJsonValue.ConstructJsonValueObject` _returnvalue) "/"))

(fn `UserConstructionScript`)