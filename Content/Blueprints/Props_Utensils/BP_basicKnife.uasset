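; Kitchen knife prop that slices procedural-mesh ingredients when its blade overlaps them.
; Cuts require CanCut, an unstacked item and bounds above a fraction of initial volume, re-arming once the blade moves far enough from the last cut.
; SliceProceduralMesh cuts along the handle's plane with a capped face.
; The new half's sections are copied into a spawned, physics-simulated BP_SubIngredient inheriting name and initial volume, with pitch-varied audio.
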(event `self.ReceiveBeginPlay`
  (set `self.LastCutPos` (0.0 0.0 0.0)))

(event `self.ReceiveTick`
  (params (DeltaSeconds :type "Float (single-precision)"))
  (if (> (`KismetMathLibrary.Vector_Distance` (`self.LastCutPos`) (`SceneComponent.K2_GetComponentLocation` (`self.blade`))) (`self.DistToReset`))
    (set `self.LastCutPos` (0.0 0.0 0.0))))

(event `self.blade.OnComponentBeginOverlap`
  (params (OverlappedComponent :type "PrimitiveComponent Object Reference") (OtherActor :type "Actor Object Reference") (OtherComp :type "PrimitiveComponent Object Reference") (OtherBodyIndex :type Integer) (bFromSweep :type Boolean) (SweepResult :type "HitResult Structure (by ref)"))
  (bind _handle (`self.handle`))
  (if (`self.CanCut`)
    (if (== (`self.LastCutPos`) (0.0 0.0 0.0))
      (set `self.LastCutPos` (`SceneComponent.K2_GetComponentLocation` (`self.blade`)))
      (bind _asprocedural_mesh_component (cast `ProceduralMeshComponent` OtherComp))
      (bind _out (`self.IsTooBigToSlice` _asprocedural_mesh_component))
      (if _out
        (for _array_element (`SceneComponent.GetChildrenComponents` OtherComp false)
          (bind _asstack_item_component (cast `/Game/Blueprints/GameplayComponents/StackItemComponent` _array_element)
            (:`then`
              (set `/Game/Blueprints/GameplayComponents/StackItemComponent.isCut` true _asstack_item_component))
            (:`CastFailed`
              (bind _asingredient_item_component (cast `/Game/Blueprints/GameplayComponents/IngredientItemComponent` _array_element))
              (set `self.IngredientName` (`/Game/Blueprints/GameplayComponents/IngredientItemComponent.IngredientName` _asingredient_item_component)))))
        (if (not (`/Game/Blueprints/GameplayComponents/StackItemComponent.isStacked` _asstack_item_component))
          (bind _outotherhalfprocmesh (`KismetProceduralMeshLibrary.SliceProceduralMesh` _asprocedural_mesh_component (`SceneComponent.K2_GetComponentLocation` _handle) (`SceneComponent.GetRightVector` _handle) true "CreateNewSectionForCap" (`PrimitiveComponent.GetMaterial` OtherComp 0)))
          (`self.PlaySound`)
          (bind _output_get (set `self.sliceHalf` _outotherhalfprocmesh))
          (`ProceduralMeshComponent.ClearCollisionConvexMeshes` _output_get)
          (bind _returnvalue (`|SpawnActorFromClass` "/Game/Blueprints/Ingredients/BP_SubIngredient.BP_SubIngredient_C" (`SceneComponent.K2_GetComponentToWorld` (`self.sliceHalf`)) "Undefined" "OverrideRootScale" null null))
          (for _array_element_2 (`SceneComponent.GetChildrenComponents` (`/Game/Blueprints/Ingredients/BP_SubIngredient.ProceduralIngredient` _returnvalue) false)
            (bind _asingredient_item_component_2 (cast `/Game/Blueprints/GameplayComponents/IngredientItemComponent` _array_element_2))
            (set `/Game/Blueprints/GameplayComponents/IngredientItemComponent.IngredientName` (`self.IngredientName`) _asingredient_item_component_2)
            (break))
          (set `/Game/Blueprints/Ingredients/BP_SubIngredient.initialVolume` (`self.Initial Volume`) _returnvalue)
          (bind _proceduralingredient (`/Game/Blueprints/Ingredients/BP_SubIngredient.ProceduralIngredient` _returnvalue))
          (`PrimitiveComponent.SetSimulatePhysics` _proceduralingredient true)
          (for _index (range (+ (`ProceduralMeshComponent.GetNumSections` (`self.sliceHalf`)) 1))
            (bind (_vertices _triangles _normals _uvs _tangents) (`KismetProceduralMeshLibrary.GetSectionFromProceduralMesh` (`self.sliceHalf`) _index))
            (`ProceduralMeshComponent.CreateMeshSection_LinearColor` :`self` _proceduralingredient :`SectionIndex` _index :`Vertices` _vertices :`Triangles` _triangles :`Normals` _normals :`UV0` _uvs :`Tangents` _tangents :`bCreateCollision` true)
            (`ProceduralMeshComponent.AddCollisionConvexMesh` _proceduralingredient _vertices)
            (`PrimitiveComponent.SetMaterial` _proceduralingredient _index (`PrimitiveComponent.GetMaterial` (`self.sliceHalf`) 0)))
          (`ProceduralMeshComponent.ClearAllMeshSections` (`self.sliceHalf`)))))))

(event `PlaySound`
  (bind _audio (`self.Audio`))
  (`AudioComponent.SetPitchMultiplier` _audio (`KismetMathLibrary.RandomFloatInRange` 0.9 1.1))
  (`AudioComponent.Play` _audio 0.0))

(fn `IsTooBigToSlice`
  (params (proceduralMesh :type "ProceduralMeshComponent Object Reference"))
  (returns (out :type Boolean))
  (bind _returnvalue (`ActorComponent.GetOwner` proceduralMesh))
  (bind _returnvalue_2 (* (* (.x (`.BoxExtent` (`KismetSystemLibrary.GetComponentBounds` proceduralMesh))) (.y (`.BoxExtent` (`KismetSystemLibrary.GetComponentBounds` proceduralMesh)))) (.z (`.BoxExtent` (`KismetSystemLibrary.GetComponentBounds` proceduralMesh)))))
  (bind _asbp_cutable (cast `/Game/Blueprints/Ingredients/BP_Cutable` _returnvalue)
    (:`then`
      (bind _initialvolume (`/Game/Blueprints/Ingredients/BP_Cutable.initialVolume` _asbp_cutable))
      (set `self.Initial Volume` _initialvolume)
      (return (> _returnvalue_2 (* _initialvolume (`self.CutSizeTreshold`)))))
    (:`CastFailed`
      (bind _asbp_sub_ingredient (cast `/Game/Blueprints/Ingredients/BP_SubIngredient` _returnvalue))
      (bind _initialvolume_2 (`/Game/Blueprints/Ingredients/BP_SubIngredient.initialVolume` _asbp_sub_ingredient))
      (set `self.Initial Volume` _initialvolume_2)
      (return (> _returnvalue_2 (* _initialvolume_2 (`self.CutSizeTreshold`)))))))

(fn `UserConstructionScript`)