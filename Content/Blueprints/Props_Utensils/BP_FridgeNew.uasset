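; VR fridge prop with a grabbable door that restocks burger ingredients when released near its closed angle.
; While grabbed, Tick turns the door's yaw toward the hand within clamped limits, and a posed hand mesh replaces the real one on the handle.
; Dropping within snap range shuts the door and calls SpawnFood, which spawns ingredients at set points, gated by a short cooldown.
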(event `SnapHandToHandle`
  (params (HandMesh :type "SceneComponent Object Reference") (isRightHand :type Boolean))
  (`SceneComponent.SetVisibility` HandMesh false true)
  (if isRightHand
    (`SceneComponent.SetVisibility` (`self.RightHandPose`) true true)
    (else
      (`SceneComponent.SetVisibility` (`self.LeftHandPose`) true true))))

(event `Grab`
  (params (HandController :type "SceneComponent Object Reference") (isRightHand :type Boolean))
  (`KismetSystemLibrary.PrintString` "Hello" true true (struct :`G` 1.0 :`B` 0.161053 :`A` 1.0) 20.0)
  (set `self.Hand` HandController)
  (set `self.isGrabbed` true)
  (set `self.isRightHand` isRightHand))

(event `Drop`
  (bind _door (`self.Door`))
  (bind (_returnvalue_roll _returnvalue_pitch _returnvalue_yaw) (`KismetMathLibrary.BreakRotator` (`SceneComponent.K2_GetComponentRotation` _door)))
  (`KismetSystemLibrary.PrintString` "Goodbye" true true (struct :`G` 1.0 :`B` 0.161053 :`A` 1.0) 20.0)
  (set `self.isGrabbed` false)
  (set `self.Hand` null)
  (if (`KismetMathLibrary.NearlyEqual_FloatFloat` _returnvalue_yaw (`self.ClosedAngle`) (`self.SnapRange`))
    (`SceneComponent.K2_SetWorldRotation` _door (`KismetMathLibrary.MakeRotator` 0.0 0.0 (`self.ClosedAngle`)) false false)
    (`self.SpawnFood`))
  (`SceneComponent.SetVisibility` (`self.RightHandPose`) false true)
  (`SceneComponent.SetVisibility` (`self.LeftHandPose`) false true))

(event `self.ReceiveTick`
  (params (DeltaSeconds :type "Float (single-precision)"))
  (`|ExecutionSequence`
    (:`then_0`
      (if (`self.isGrabbed`)
        (bind _hand (`self.Hand`)
          (:`then`
            (bind (_returnvalue_roll _returnvalue_pitch _returnvalue_yaw) (`KismetMathLibrary.BreakRotator` (`KismetMathLibrary.FindLookAtRotation` (`SceneComponent.K2_GetComponentLocation` _hand) (`SceneComponent.K2_GetComponentLocation` (`self.Door`)))))
            (`SceneComponent.K2_SetWorldRotation` (`self.Door`) (`KismetMathLibrary.MakeRotator` 0.0 0.0 (`KismetMathLibrary.ClampAngle` (- _returnvalue_yaw (`self.WorldRotatationCorrection`)) (`self.MinAngle`) (`self.MaxAngle`))) false false))
          (:`else`))))
    (:`then_1`
      (set `self.SpawnCooldown` (- (`self.SpawnCooldown`) DeltaSeconds)))))

(event `SpawnFood`
  (bind _returnvalue (`SceneComponent.K2_GetComponentToWorld` (`self.baconPoint`)))
  (if (<= (`self.SpawnCooldown`) 0.0)
    (`|ExecutionSequence`
      (:`then_0`
        (`|SpawnActorFromClass` "/Game/Blueprints/Ingredients/Steak/BP_Steak.BP_Steak_C" (`SceneComponent.K2_GetComponentToWorld` (`self.steakPoint`)) "Undefined" "OverrideRootScale" null null))
      (:`then_1`
        (`|SpawnActorFromClass` "/Game/Blueprints/Ingredients/Bread/BP_Bread_Top.BP_Bread_Top_C" (`SceneComponent.K2_GetComponentToWorld` (`self.breadTopPoint`)) "Undefined" "OverrideRootScale" null null))
      (:`then_2`
        (`|SpawnActorFromClass` "/Game/Blueprints/Ingredients/Bread/BP_Bread_Bottom.BP_Bread_Bottom_C" (`SceneComponent.K2_GetComponentToWorld` (`self.breadBottomPoint`)) "Undefined" "OverrideRootScale" null null))
      (:`then_3`
        (`|SpawnActorFromClass` "/Game/Blueprints/Ingredients/Cheese/BP_CheeseSimple.BP_CheeseSimple_C" (`SceneComponent.K2_GetComponentToWorld` (`self.cheesePoint`)) "Undefined" "OverrideRootScale" null null))
      (:`then_4`
        (`|SpawnActorFromClass` "/Game/Blueprints/Ingredients/Onion/BP_Onion.BP_Onion_C" (`SceneComponent.K2_GetComponentToWorld` (`self.onionPoint`)) "Undefined" "OverrideRootScale" null null))
      (:`then_5`
        (switch `int` (`KismetMathLibrary.RandomIntegerInRange` 0 2)
          (:`0`
            (`|SpawnActorFromClass` "/Game/Blueprints/Ingredients/Bacon/BP_Bacon.BP_Bacon_C" _returnvalue "Undefined" "OverrideRootScale" null null))
          (:`1`
            (`|SpawnActorFromClass` "/Game/Blueprints/Ingredients/Bacon/BP_Bacon2.BP_Bacon2_C" _returnvalue "Undefined" "OverrideRootScale" null null))
          (:`2`
            (`|SpawnActorFromClass` "/Game/Blueprints/Ingredients/Bacon/BP_Bacon3.BP_Bacon3_C" _returnvalue "Undefined" "OverrideRootScale" null null))))
      (:`then_6`
        (`|SpawnActorFromClass` "/Game/Blueprints/Ingredients/BP_Tomato.BP_Tomato_C" (`SceneComponent.K2_GetComponentToWorld` (`self.tomatoPoint`)) "Undefined" "OverrideRootScale" null null))
      (:`then_7`
        (set `self.SpawnCooldown` 2.0)))))

(fn `UserConstructionScript`
  (set `self.SpawnCooldown` 2.0))