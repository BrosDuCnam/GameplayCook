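; Fridge prop with a hinged door that follows a grabbing hand within angle limits.
; Pickup and drop events store or clear the hand component and open or close a Tick gate.
; While tracking, the hand's flattened direction from the door gives a signed angle against the starting right vector, selecting a clamped or hand-following rotation, with constant-rate interpolation helpers.
; A helper to snap the hand to the handle socket is defined but not called here.
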(event `self.ReceiveBeginPlay`
  ;[1 1 1] Get initial door right vector, used to compute door angle
  (set `self.InitDoorDirection` (`SceneComponent.GetRightVector` (`self.Door`))))

(event `EventPickUp`
  (params (Component :type "SceneComponent Object Reference") (Hand :type "EControllerHand Enum" :default "Left"))
  ;[1 1 1] Pick up and drop
  (`KismetSystemLibrary.PrintString` "Hello" true true (struct :`R` 0.042262 :`G` 1.0 :`A` 1.0) 20.0)
  (set `self.Hand` Component)
  (`self.StartTracking`))

(event `EventDrop`
  (params (Component :type "SceneComponent Object Reference"))
  ;[1 1 1] Pick up and drop
  (`KismetSystemLibrary.PrintString` "Goodbye" true true (struct :`R` 1.0 :`G` 0.497199 :`A` 1.0) 20.0)
  (`self.StopTracking`)
  (set `self.Hand` null))

(event `self.ReceiveTick`
  (params (DeltaSeconds :type "Float (single-precision)"))
  (`/Engine/EditorBlueprintResources/StandardMacros.Gate` true :!label _label
    (:`Exit`
      (set `self.CurrentAngle` (`self.GetDoorAngle`)) ; Get the current door angle compared to its starting\nright vector.
      ;[1 1 1] Set the door rotation based on the clamped angle
      (if (>= (`self.CurrentAngle`) (`self.MinAngle`))
        (`SceneComponent.K2_SetRelativeRotation` (`self.Door`) (`KismetMathLibrary.RInterpTo_Constant` (`SceneComponent.RelativeRotation` (`self.Door`)) (`self.GetDoorRotation` (`self.InitDoorDirection`) true) (`GameplayStatics.GetWorldDeltaSeconds`) 100.0) false false)
        (elif (<= (`self.CurrentAngle`) (`self. MaxAngle`))
          (`SceneComponent.K2_SetRelativeRotation` (`self.Door`) (`KismetMathLibrary.RInterpTo_Constant` (`SceneComponent.RelativeRotation` (`self.Door`)) (`self.GetDoorRotation` (`KismetMathLibrary.RotateAngleAxis` (`self.InitDoorDirection`) (`self. MaxAngle`) (`KismetMathLibrary.NegateVector` (`SceneComponent.GetUpVector` (`self.Door`)))) true) (`GameplayStatics.GetWorldDeltaSeconds`) 100.0) false false)
          (else
            (`SceneComponent.K2_SetRelativeRotation` (`self.Door`) (`KismetMathLibrary.RInterpTo_Constant` (`SceneComponent.RelativeRotation` (`self.Door`)) (`self.GetDoorRotation` (`self.InitDoorDirection`)) (`GameplayStatics.GetWorldDeltaSeconds`) 100.0) false false)))))))

(event `StartTracking`
  (goto _label :!via `Open`))

(event `StopTracking`
  (goto _label :!via `Close`))

(fn `GetDoorAngle`
  (returns (ReturnValue :type "Float (double-precision)"))
  (bind (_returnvalue_x _returnvalue_y _returnvalue_z) (`KismetMathLibrary.BreakVector` (`KismetMathLibrary.Cross_VectorVector` (`self.GetHandDoorDirection`) (`self.InitDoorDirection`))))
  (return (* (`KismetMathLibrary.DegAcos` (`KismetMathLibrary.Dot_VectorVector` (`self.GetHandDoorDirection`) (`self.InitDoorDirection`))) (`KismetMathLibrary.SelectFloat` -1.0 1.0 (< _returnvalue_z 0.0)))))

(fn `GetDoorRotation`
  (params (OptionalDirection :type "Vector Structure") (UseDirection :type Boolean))
  (returns (ReturnValue :type "Rotator Structure"))
  (return (`KismetMathLibrary.MakeRotFromYZ` (`KismetMathLibrary.SelectVector` OptionalDirection (`self.GetHandDoorDirection`) UseDirection) (`SceneComponent.GetUpVector` (`self.Door`)))))

(fn `GetHandDoorDirection`
  (returns (ReturnValue :type "Vector Structure"))
  (return (`KismetMathLibrary.Normal` (`KismetMathLibrary.MakeVector` (.x (- (`SceneComponent.K2_GetComponentLocation` (`self.Hand`)) (`SceneComponent.K2_GetComponentLocation` (`self.Door`)))) (.y (- (`SceneComponent.K2_GetComponentLocation` (`self.Hand`)) (`SceneComponent.K2_GetComponentLocation` (`self.Door`))))))))

(fn `SnapHandToHandle`
  (params (Hand :type "SceneComponent Object Reference"))
  (`SceneComponent.K2_SetWorldLocationAndRotation` Hand (`SceneComponent.GetSocketLocation` (`self.Door`) "Handle_Socket") (`SceneComponent.GetSocketRotation` (`self.Door`) "Handle_Socket") false true))

(fn `UserConstructionScript`)