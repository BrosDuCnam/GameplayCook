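; BP_ScoreDisplay is a Blueprint that shows a score on a text render component, updated by socket events.
; On BeginPlay it reaches the Socket.IO client through BP_GameInstance and binds UpdateScore to the "score_updated" event.
; UpdateScore reads the numeric "message" field from the event's JSON, stores it truncated as an integer in Score and writes it to the text.
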(event `self.ReceiveBeginPlay`
  (`SocketIOClientComponent.BindEventToDelegate` (`/Game/Blueprints/ServerStuff/BP_Client.SIOClient` (`/Game/Blueprints/ServerStuff/BP_GameInstance.Client` (cast `/Game/Blueprints/ServerStuff/BP_GameInstance` (`GameplayStatics.GetGameInstance`) :!pure true))) "score_updated" (delegate `UpdateScore`) "/" "USE_DEFAULT"))

(event `UpdateScore`
  (params (EventData :type "SIOJsonValue Object Reference"))
  (bind _returnvalue (`KismetMathLibrary.FTrunc` (`SIOJsonObject.GetNumberField` (`SIOJLibrary.Conv_JsonValueToJsonObject` EventData) "message")))
  (set `self.Score` _returnvalue)
  (`TextRenderComponent.K2_SetText` (`self.TextRender`) (`KismetTextLibrary.Conv_IntToText` _returnvalue)))

(fn `UserConstructionScript`)