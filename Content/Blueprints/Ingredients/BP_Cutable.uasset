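; BP_Cutable is an ingredient actor set up as a procedural mesh, apparently so it can be cut.
; Its construction script applies the configured mesh and material to a static mesh component, then copies that into a procedural mesh component.
; Vertices from the mesh's first LOD 0 section become convex collision.
; It stores an initial volume as the product of the procedural mesh's bounds extents; the event graph is empty.
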(fn `UserConstructionScript`
  (bind _staticingredient (`self.StaticIngredient`))
  (bind _proceduralingredient (`self.ProceduralIngredient`))
  (`StaticMeshComponent.SetStaticMesh` _staticingredient (`self.Ingredient`))
  (`PrimitiveComponent.SetMaterial` _staticingredient 0 (`self.IngredientMaterial`))
  (`KismetProceduralMeshLibrary.CopyProceduralMeshFromStaticMeshComponent` _staticingredient 0 _proceduralingredient)
  (bind _vertices (`KismetProceduralMeshLibrary.GetSectionFromStaticMesh` (`self.Ingredient`)))
  (`ProceduralMeshComponent.AddCollisionConvexMesh` _proceduralingredient _vertices)
  (set `self.initialVolume` (* (* (.x (`.BoxExtent` (`KismetSystemLibrary.GetComponentBounds` (`self.ProceduralIngredient`)))) (.y (`.BoxExtent` (`KismetSystemLibrary.GetComponentBounds` (`self.ProceduralIngredient`))))) (.z (`.BoxExtent` (`KismetSystemLibrary.GetComponentBounds` (`self.ProceduralIngredient`)))))))