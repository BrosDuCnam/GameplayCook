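; BP_Thrower is a grabbable launcher that fires balls at a fixed interval while it is held.
; A looping timer started on BeginPlay calls Throw, which checks the GrabComponent's held state before acting.
; Each throw spawns a Bp_ThrowerBall at the Arrow component's transform and pushes its sphere forward with an impulse scaled by Force.
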(event `self.ReceiveBeginPlay`
  (`KismetSystemLibrary.K2_SetTimerDelegate` (delegate `Throw`) (`self.Timer`) true))

(event `Throw`
  (if (`/Game/VRTemplate/Blueprints/GrabComponent.bIsHeld` (`self.GrabComponent`))
    (bind _returnvalue (`|SpawnActorFromClass` "/Game/Blueprints/Thrower/Bp_ThrowerBall.Bp_ThrowerBall_C" (`SceneComponent.K2_GetComponentToWorld` (`self.Arrow`)) "Undefined" "OverrideRootScale" null null))
    (`PrimitiveComponent.AddImpulse` (`/Game/Blueprints/Thrower/Bp_ThrowerBall.Sphere` _returnvalue) (* (`SceneComponent.GetForwardVector` (`self.Arrow`)) (`self.Force`)) "None" false)))

(fn `UserConstructionScript`)