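; BP_CityNightTemp is an actor that repositions itself from a "kitchen_pos" Socket.IO message.
; A looping timer polls the game instance's SocketIO client until it connects, then stops and binds SetPos to that event.
; SetPos prints the JSON payload and position, then applies its location and yaw to the actor.
; The construction script disables collision on all static mesh components under the scene root.
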(event `self.ReceiveBeginPlay`
  (bind _returnvalue (`KismetSystemLibrary.K2_SetTimerDelegate` (delegate `check_connect`) 1.0 true)))

(event `check_connect`
  (bind _sioclient (`/Game/Blueprints/ServerStuff/BP_Client.SIOClient` (`/Game/Blueprints/ServerStuff/BP_GameInstance.Client` (cast `/Game/Blueprints/ServerStuff/BP_GameInstance` (`GameplayStatics.GetGameInstance`) :!pure true))))
  (if (`SocketIOClientComponent.bIsConnected` _sioclient)
    (`KismetSystemLibrary.K2_ClearAndInvalidateTimerHandle` (stale `self.ReceiveBeginPlay` _returnvalue))
    (`SocketIOClientComponent.BindEventToDelegate` _sioclient "kitchen_pos" (delegate `SetPos`) "/" "USE_DEFAULT")))

(event `SetPos`
  (params (EventData :type "SIOJsonValue Object Reference"))
  (bind _returnvalue (`SIOJLibrary.Conv_JsonValueToJsonObject` EventData))
  (bind _returnvalue_2 (`SIOJsonObject.GetObjectField` _returnvalue "message"))
  (bind _returnvalue_3 (`KismetMathLibrary.MakeVector` (`SIOJsonObject.GetNumberField` _returnvalue_2 "x") (`SIOJsonObject.GetNumberField` _returnvalue_2 "y") (`SIOJsonObject.GetNumberField` _returnvalue_2 "z")))
  (`KismetSystemLibrary.PrintString` (`SIOJLibrary.Conv_SIOJsonObjectToString` _returnvalue))
  (`KismetSystemLibrary.PrintString` (`KismetStringLibrary.Conv_VectorToString` _returnvalue_3))
  (`self.K2_SetActorLocationAndRotation` _returnvalue_3 (`KismetMathLibrary.MakeRotator` 0.0 0.0 (`SIOJsonObject.GetNumberField` _returnvalue_2 "rotation"))))

(fn `UserConstructionScript`
  (for _array_element (`SceneComponent.GetChildrenComponents` (`self.DefaultSceneRoot`) true)
    (bind _asstatic_mesh_component (cast `StaticMeshComponent` _array_element))
    (`PrimitiveComponent.SetCollisionEnabled` _asstatic_mesh_component "NoCollision")))