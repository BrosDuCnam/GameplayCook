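; Collision box that reports objects thrown into it to a Socket.IO server.
; A hit or overlap, gated by a half-second cooldown, captures the object's box-relative location and velocity, then emits them with ingredients from the order-completed area.
; Server events toggle root visibility for the kitchen's open state and track truck angle, with only a debug print on sharp turns at speed.
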(event `self.ReceiveBeginPlay`
  (bind _output_get (set `self.client` (`/Game/Blueprints/ServerStuff/BP_Client.SIOClient` (`/Game/Blueprints/ServerStuff/BP_GameInstance.Client` (cast `/Game/Blueprints/ServerStuff/BP_GameInstance` (`GameplayStatics.GetGameInstance`) :!pure true)))))
  (`SocketIOClientComponent.BindEventToFunction` _output_get "set_kitchen_pos" "update_kitchen" self "/" "USE_DEFAULT")
  (`SocketIOClientComponent.BindEventToFunction` _output_get "set_velocity" "update_velocity" null "/" "USE_DEFAULT"))

(event `self.Cube.OnComponentHit`
  (params (HitComponent :type "PrimitiveComponent Object Reference") (OtherActor :type "Actor Object Reference") (OtherComp :type "PrimitiveComponent Object Reference") (NormalImpulse :type "Vector Structure") (Hit :type "HitResult Structure (by ref)"))
  (`|ExecutionSequence` :!label _label
    (:`then_0`
      (if (`self.CanReceive`)
        (set `self.CanReceive` false)
        (set `self.CollisionObject` (`ActorComponent.GetOwner` (stale `self.Cube.OnComponentBeginOverlap` OtherComp)))
        (bind _output_get (set `self.CollisionLocation` (/ (+ (/ (/ (- (`SceneComponent.K2_GetComponentLocation` (stale `self.Cube.OnComponentBeginOverlap` OtherComp)) (`SceneComponent.K2_GetComponentLocation` (`self.DefaultSceneRoot`))) (`SceneComponent.K2_GetComponentScale` (`self.Cube`))) 100.0) 1.5) 2.0)))
        (bind _output_get_2 (set `self.CollisionVelocity` (`SceneComponent.GetComponentVelocity` (stale `self.Cube.OnComponentBeginOverlap` OtherComp))))
        (`KismetSystemLibrary.PrintString` (`KismetStringLibrary.Concat_StrStr` "Location: " (`KismetStringLibrary.Conv_VectorToString` _output_get) " - Velocity: " (`KismetStringLibrary.Conv_VectorToString` _output_get_2)))
        (`self.SendCollisionInfo`)))
    (:`then_1`
      (`KismetSystemLibrary.Delay` 0.5)
      (set `self.CanReceive` true))))

(event `self.Cube.OnComponentBeginOverlap`
  (params (OverlappedComponent :type "PrimitiveComponent Object Reference") (OtherActor :type "Actor Object Reference") (OtherComp :type "PrimitiveComponent Object Reference") (OtherBodyIndex :type Integer) (bFromSweep :type Boolean) (SweepResult :type "HitResult Structure (by ref)"))
  (goto _label))

(fn `SendCollisionInfo`
  (bind _returnvalue (`self.GetComponentByClass` (`self.CollisionObject`) "/Game/Blueprints/GameplayComponents/StackItemComponent.StackItemComponent_C"))
  (bind _returnvalue_2 (`SIOJsonObject.ConstructJsonObject`))
  (`SIOJsonObject.SetStringField` _returnvalue_2 "object_name" (`KismetStringLibrary.Conv_ObjectToString` (`self.CollisionObject`)))
  (`SIOJsonObject.SetArrayField` _returnvalue_2 "location" (`self.VectorToJsonArray` (`self.CollisionLocation`)))
  (`SIOJsonObject.SetArrayField` _returnvalue_2 "velocity" (`self.VectorToJsonArray` (`self.CollisionVelocity`)))
  (`KismetSystemLibrary.PrintString` (`KismetSystemLibrary.GetDisplayName` _returnvalue))
  (bind _messagearray (`/Game/Blueprints/GameplayComponents/OrderCompletedAreaComponent.OnOrderCompleted` (`self.OrderCompletedAreaComponent`) _returnvalue))
  (`SIOJsonObject.SetStringArrayField` _returnvalue_2 "ingredients" _messagearray)
  (bind _returnvalue_3 (`SIOJsonValue.ConstructJsonValueObject` _returnvalue_2))
  (`KismetSystemLibrary.PrintString` (`SIOJLibrary.Conv_SIOJsonObjectToString` (`SIOJLibrary.Conv_JsonValueToJsonObject` _returnvalue_3)) true true (struct :`R` 1.0 :`G` 0.026519 :`A` 1.0) 100.0)
  (`SocketIOClientComponent.Emit` (`self.client`) "on_object_thrown" _returnvalue_3 "/"))

(fn `update_kitchen`
  (params (json :type "SIOJsonObject Object Reference"))
  (`SceneComponent.SetVisibility` (`self.DefaultSceneRoot`) (`SIOJsonObject.GetBoolField` json "open") false))

(fn `update_velocity`
  (params (json :type "SIOJsonObject Object Reference"))
  (bind _returnvalue (`SIOJsonObject.GetNumberField` json "angle"))
  (`|ExecutionSequence`
    (:`then_0`
      (if (and (> (`SIOJsonObject.GetNumberField` json "speed") 50.0) (!= (`self.truckAngle`) -900.0))
        (if (> (`KismetMathLibrary.Abs` (- (`self.truckAngle`) _returnvalue)) 15.0)
          (`KismetSystemLibrary.PrintString` "I Believe i can fly"))))
    (:`then_1`
      (set `self.truckAngle` _returnvalue))))

(fn `UserConstructionScript`)