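; BP_Command_manager receives new orders from a Socket.IO server and spawns a BP_Command actor for each one.
; On BeginPlay a looping timer polls the game instance's client until it connects, then clears itself and binds the "new_order" event to new_command.
; That handler prints the JSON message, spawns the actor at a hardcoded transform and passes it the order's id and ingredient list.
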(event `self.ReceiveBeginPlay`
  (bind _returnvalue (`KismetSystemLibrary.K2_SetTimerDelegate` (delegate `check_connect`) 1.0 true)))

(event `check_connect`
  (bind _sioclient (`/Game/Blueprints/ServerStuff/BP_Client.SIOClient` (`/Game/Blueprints/ServerStuff/BP_GameInstance.Client` (cast `/Game/Blueprints/ServerStuff/BP_GameInstance` (`GameplayStatics.GetGameInstance`) :!pure true))))
  (if (`SocketIOClientComponent.bIsConnected` _sioclient)
    (`KismetSystemLibrary.K2_ClearAndInvalidateTimerHandle` (stale `self.ReceiveBeginPlay` _returnvalue))
    (`SocketIOClientComponent.BindEventToFunction` _sioclient "new_order" "new_command" self "/" "USE_DEFAULT")))

(fn `new_command`
  (params (data :type "SIOJsonObject Object Reference"))
  (bind _returnvalue (`SIOJsonObject.GetObjectField` data "message"))
  (bind _returnvalue_2 (`SIOJsonObject.GetStringArrayField` _returnvalue "ingredients"))
  (`KismetSystemLibrary.PrintString` (`SIOJLibrary.Conv_SIOJsonObjectToString` _returnvalue))
  (bind _returnvalue_3 (`|SpawnActorFromClass` "/Game/Blueprints/ServerStuff/BP_Command.BP_Command_C" (`KismetMathLibrary.MakeTransform` (-5.0 73.0 109.0) (struct :`Yaw` 180.0)) "Undefined" "OverrideRootScale" null null))
  (`/Game/Blueprints/ServerStuff/BP_Command.set_command` _returnvalue_3 (`KismetStringLibrary.Conv_Int64ToString` (`KismetMathLibrary.FTrunc64` (`SIOJsonObject.GetNumberField` _returnvalue "id"))) _returnvalue_2)
  (return))

(fn `UserConstructionScript`)