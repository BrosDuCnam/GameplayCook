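; BP_Command is an actor that displays a numbered command, likely an order, with its list of ingredients as text.
; SetCommand writes the Id prefixed with "#" into the TextId component.
; It then builds one string from an "Ingredients:" header plus each ingredient behind a dash and pushes it to TextIngredient.
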(fn `set_command`
  (params (id :type String) (ingredients :type "Array of String"))
  (locals (text :type String))
  (set `local.text` "Ingredients: \n")
  (`TextRenderComponent.K2_SetText` (`self.text_id`) (`KismetTextLibrary.Conv_StringToText` (`KismetStringLibrary.Concat_StrStr` "# " id)))
  (for _array_element ingredients
    (set `local.text` (`KismetStringLibrary.Concat_StrStr` (`local.text`) "-  " _array_element " \n")))
  (`TextRenderComponent.K2_SetText` (`self.text_ingredient`) (`KismetTextLibrary.Conv_StringToText` (`local.text`)))
  (return))

(fn `UserConstructionScript`)