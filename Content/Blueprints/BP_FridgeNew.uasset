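; BP_FridgeNew is a fridge whose door swings open and closed when grabbed by a hand controller, apparently for VR.
; While grabbed, Tick yaws the door from the look-at rotation between hand and door, offset by a correction and clamped to angle limits.
; SnapHandToHandle swaps the hand mesh for a left or right handle pose.
; Drop hides both poses and snaps the door shut when within range of its closed angle.
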(event `SnapHandToHandle`
  (params (HandMesh :type "SceneComponent Object Reference") (isRightHand :type Boolean))
  (`SceneComponent.SetVisibility` HandMesh false true)
  (if isRightHand
    (`SceneComponent.SetVisibility` (`self.RightHandPose`) true true)
    (else
      (`SceneComponent.SetVisibility` (`self.LeftHandPose`) true true))))

(event `Grab`
  (params (HandController :type "SceneComponent Object Reference") (isRightHand :type Boolean))
  (`KismetSystemLibrary.PrintString` "Hello" true true (struct :`G` 1.0 :`B` 0.161053 :`A` 1.0) 20.0)
  (set `self.Hand` HandController)
  (set `self.isGrabbed` true)
  (set `self.isRightHand` isRightHand))

(event `Drop`
  (bind _door (`self.Door`))
  (bind (_returnvalue_roll _returnvalue_pitch _returnvalue_yaw) (`KismetMathLibrary.BreakRotator` (`SceneComponent.K2_GetComponentRotation` _door)))
  (`KismetSystemLibrary.PrintString` "Goodbye" true true (struct :`G` 1.0 :`B` 0.161053 :`A` 1.0) 20.0)
  (set `self.isGrabbed` false)
  (set `self.Hand` null)
  (if (`KismetMathLibrary.NearlyEqual_FloatFloat` _returnvalue_yaw (`self.ClosedAngle`) (`self.SnapRange`))
    (`SceneComponent.K2_SetWorldRotation` _door (`KismetMathLibrary.MakeRotator` 0.0 0.0 (`self.ClosedAngle`)) false false))
  (`SceneComponent.SetVisibility` (`self.RightHandPose`) false true)
  (`SceneComponent.SetVisibility` (`self.LeftHandPose`) false true))

(event `self.ReceiveTick`
  (params (DeltaSeconds :type "Float (single-precision)"))
  (if (`self.isGrabbed`)
    (bind _hand (`self.Hand`)
      (:`then`
        (bind (_returnvalue_roll _returnvalue_pitch _returnvalue_yaw) (`KismetMathLibrary.BreakRotator` (`KismetMathLibrary.FindLookAtRotation` (`SceneComponent.K2_GetComponentLocation` _hand) (`SceneComponent.K2_GetComponentLocation` (`self.Door`)))))
        (`SceneComponent.K2_SetWorldRotation` (`self.Door`) (`KismetMathLibrary.MakeRotator` 0.0 0.0 (`KismetMathLibrary.ClampAngle` (- _returnvalue_yaw (`self.WorldRotatationCorrection`)) (`self.MinAngle`) (`self.MaxAngle`))) false false))
      (:`else`))))

(fn `UserConstructionScript`)