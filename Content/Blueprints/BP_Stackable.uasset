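; BP_Stackable fits top and bottom cylinder markers to its static mesh, apparently as attachment zones for stacking.
; On BeginPlay it reads the local bounds of the first StaticMeshComponent, taking width as the XY diagonal and height as the Z extent.
; Both cylinders get a world scale from the reciprocals of those sizes and move to the bottom and top Z bounds.
; The file contains no stacking logic.
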(event `self.ReceiveBeginPlay`
  (bind _returnvalue (/ 1.0 (`self.Width`)))
  (bind _returnvalue_2 (`self.K2_GetComponentsByClass` (`ActorComponent.GetOwner` (`self.DefaultSceneRoot`)) "/Script/Engine.StaticMeshComponent"))
  (bind (_min _max) (`StaticMeshComponent.GetLocalBounds` (`|GetArrayItem` _returnvalue_2)))
  (if (> (`KismetArrayLibrary.Array_Length` _returnvalue_2) 0)
    (set `self.Width` (`KismetMathLibrary.Distance2D` (`KismetMathLibrary.MakeVector2D` (.x _min) (.y _min)) (`KismetMathLibrary.MakeVector2D` (.x _max) (.y _max))))
    (set `self.Height` (- (.z _max) (.z _min)))
    (`SceneComponent.SetWorldScale3D` (`self.BotCylinder`) (`KismetMathLibrary.MakeVector` _returnvalue _returnvalue (/ 1.0 (`self.Height`))))
    (`SceneComponent.SetWorldScale3D` (`self.TopCylinder`) (`SceneComponent.K2_GetComponentScale` (`self.BotCylinder`)))
    (`SceneComponent.K2_SetRelativeLocation` (`self.BotCylinder`) (`KismetMathLibrary.MakeVector` 0.0 0.0 (.z _min)) false true)
    (`SceneComponent.K2_SetRelativeLocation` (`self.TopCylinder`) (`KismetMathLibrary.MakeVector` 0.0 0.0 (.z _max)) false true)))

(fn `UserConstructionScript`)