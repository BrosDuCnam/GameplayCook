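; BP_ClientUser is a test-style Socket.IO client Blueprint that exercises the connection held by BP_GameInstance.
; On BeginPlay it casts to the game instance and binds to its Client's SIOClientComponent connected event.
; On connection it prints the session ID and emits "Create" twice, with separate callbacks that each print the returned success value.
; The construction script and SetGaMeInstance function are empty.
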(event `self.ReceiveBeginPlay`
  (bind _asbp_game_instance (cast `/Game/BP_GameInstance` (`GameplayStatics.GetGameInstance`)))
  (add `SocketIOClientComponent.OnConnected` (`Client.SIOClientComponent` (`/Game/BP_GameInstance.Client` _asbp_game_instance)) (delegate `a`)))

(event `Print Success`
  (params (callbackStruct :type "CallbackStruct Structure"))
  (`KismetSystemLibrary.PrintString` (`KismetStringLibrary.Conv_BoolToString` callbackStruct_success) true true (struct :`G` 0.66 :`B` 1.0 :`A` 1.0) 5.0))

(event `AAA`
  (params (callbackStruct :type "CallbackStruct Structure"))
  (`KismetSystemLibrary.PrintString` (`KismetStringLibrary.Conv_BoolToString` callbackStruct_success) true true (struct :`G` 0.66 :`B` 1.0 :`A` 1.0) 5.0))

(event `a`
  (params (SocketId :type String) (SessionId :type String) (bIsReconnection :type Boolean))
  (`KismetSystemLibrary.PrintString` SessionId)
  (bind _client (`/Game/BP_GameInstance.Client` (stale `self.ReceiveBeginPlay` _asbp_game_instance)))
  (`Client.Emit` _client "Create" null (delegate `Print Success`))
  (`Client.Emit` _client "Create" null (delegate `AAA`))
  (`KismetSystemLibrary.PrintString` "AAAHello"))

(fn `Set GaMe Instance`)

(fn `UserConstructionScript`)